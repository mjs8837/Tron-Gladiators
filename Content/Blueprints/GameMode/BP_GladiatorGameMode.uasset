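; Game mode for a two-player gladiator game that sets up both players when play begins.
; It spawns an extra BP_Player, waits briefly, then gathers all players and moves them to the first two PlayerStarts by array index.
; Each player gets its own mesh material and a color choice index read from BP_GameInstance.
; EndGame is a placeholder that only prints a debug message.
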(event EventBeginPlay
  (bind _returnvalue (Game|GetGameInstance))
  ;[1 1 1] Getting player start refs to set spawns.
  (bind _outactors (Actor|GetAllActorsOfClass "/Script/Engine.PlayerStart"))
  (Variables|Default|SetplayerStarts _outactors)
  ;[1 1 1] Spawning a new player and setting players references.
  (Game|SpawnActorfromClass "/Game/Blueprints/Player/BP_Player.BP_Player_C" (Math|Transform|MakeTransform "1000.000000,1950.000000,90.000000" "0, 0, 0" "1.000000,1.000000,1.000000") "AlwaysSpawn" "MultiplyWithRoot" 0 0)
  (Utilities|FlowControl|Delay 0.2)
  (bind _outactors_2 (Actor|GetAllActorsOfClass "/Game/Blueprints/Player/BP_Player.BP_Player_C"))
  (bind _output_get (Variables|Default|Setplayers _outactors_2))
  ;[1 1 1] Setting player refs to spawn at different player starts.
  (for (_array_element _array_index) _output_get
    (if (== _array_index 0)
      (Transformation|SetActorLocation _array_element (Transformation|GetActorLocation (Utilities|Array|Get(acopy) (Variables|Default|GetplayerStarts))) false false)
      ;[1 1 1] Setting material of both players.
      (Rendering|Material|SetMaterial (Variables|/Game/Blueprints/Player/BP_Player.BP_Player_C|GetSM_PlayerMesh (Utilities|Array|Get(acopy) (Variables|Default|Getplayers))) 0 "/Game/Blueprints/Materials/M_Player0Mat.M_Player0Mat")
      (bind _asbp_game_instance (Utilities|Casting|CastToBP_GameInstance _returnvalue))
      (Variables|/Game/Blueprints/Player/BP_Player.BP_Player_C|SetcolorChoiceIndex (Utilities|Array|Get(acopy) (Variables|Default|Getplayers)) (Variables|/Game/Blueprints/BP_GameInstance.BP_GameInstance_C|Getplayer0ColorChoice _asbp_game_instance))
      (else
        (Transformation|SetActorLocation _array_element (Transformation|GetActorLocation (Utilities|Array|Get(acopy) (Variables|Default|GetplayerStarts) 1)) false false)
        (Rendering|Material|SetMaterial (Variables|/Game/Blueprints/Player/BP_Player.BP_Player_C|GetSM_PlayerMesh (Utilities|Array|Get(acopy) (Variables|Default|Getplayers) 1)) 0 "/Game/Blueprints/Materials/M_Player1Mat.M_Player1Mat")
        (bind _asbp_game_instance_2 (Utilities|Casting|CastToBP_GameInstance _returnvalue))
        (Variables|/Game/Blueprints/Player/BP_Player.BP_Player_C|SetcolorChoiceIndex (Utilities|Array|Get(acopy) (Variables|Default|Getplayers) 1) (Variables|/Game/Blueprints/BP_GameInstance.BP_GameInstance_C|Getplayer1ColorChoice _asbp_game_instance_2))))))

(fn ConstructionScript)

(fn EndGame
  (Development|PrintString "End game called from game mode."))