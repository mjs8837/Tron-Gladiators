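; Player controller that drives two local BP_Player pawns from one keyboard.
; After a short BeginPlay delay it gathers the players and player starts, moves the players to separate starts and adds the Enhanced Input mapping context.
; WASD and Left Shift move and dash the first player, while arrows and Right Shift do the same for the second.
; Tick caches delta time, which is passed into each Move call.
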(event Input|EnhancedActionEvents|EnhancedInputActionIA_MoveWASD
  (params (ActionValue :type Vector%202D%20Structure) (ElapsedSeconds :type Float%20%28double-precision%29) (TriggeredSeconds :type Float%20%28double-precision%29) (InputAction :type Input%20Action%20Object%20Reference :default "/Game/Blueprints/Player/Input/InputActions/IA_MoveWASD.IA_MoveWASD"))
  (bind (_x _y) (Math|Vector2D|BreakVector2D ActionValue))
  (bind _players (Variables|Default|Getplayers))
  (bind _output (Utilities|Array|Get(acopy) _players))
  ;[1 1 1] Handling player 0 movement with WASD
  (:Triggered
    (Variables|/Game/Blueprints/Player/BP_Player.BP_Player_C|SetmoveDirection _output (Math|Vector|MakeVector _x _y 0.0))
    (Default|Move _output (Variables|Default|GetdeltaTime)))
  (:Completed
    (Variables|/Game/Blueprints/Player/BP_Player.BP_Player_C|SetmoveDirection _output "0, 0, 0")))

(event Input|EnhancedActionEvents|EnhancedInputActionIA_MoveArrows
  (params (ActionValue :type Vector%202D%20Structure) (ElapsedSeconds :type Float%20%28double-precision%29) (TriggeredSeconds :type Float%20%28double-precision%29) (InputAction :type Input%20Action%20Object%20Reference :default "/Game/Blueprints/Player/Input/InputActions/IA_MoveArrows.IA_MoveArrows"))
  (bind (_x _y) (Math|Vector2D|BreakVector2D ActionValue))
  (bind _players (Variables|Default|Getplayers))
  (bind _output (Utilities|Array|Get(acopy) _players 1))
  ;[1 1 1] Handling player 1 movement with Arrows
  (:Triggered
    (Variables|/Game/Blueprints/Player/BP_Player.BP_Player_C|SetmoveDirection _output (Math|Vector|MakeVector _x _y 0.0))
    (Default|Move _output (Variables|Default|GetdeltaTime)))
  (:Completed
    (Variables|/Game/Blueprints/Player/BP_Player.BP_Player_C|SetmoveDirection _output "0, 0, 0")))

(event Input|EnhancedActionEvents|EnhancedInputActionIA_DashLeftShift
  (params (ActionValue :type Boolean) (ElapsedSeconds :type Float%20%28double-precision%29) (TriggeredSeconds :type Float%20%28double-precision%29) (InputAction :type Input%20Action%20Object%20Reference :default "/Game/Blueprints/Player/Input/InputActions/IA_DashLeftShift.IA_DashLeftShift"))
  ;[1 1 1] Handling dash for player 0.
  (:Triggered
    (Default|Dash (Utilities|Array|Get(acopy) (Variables|Default|Getplayers)))))

(event Input|EnhancedActionEvents|EnhancedInputActionIA_DashRightShift
  (params (ActionValue :type Boolean) (ElapsedSeconds :type Float%20%28double-precision%29) (TriggeredSeconds :type Float%20%28double-precision%29) (InputAction :type Input%20Action%20Object%20Reference :default "/Game/Blueprints/Player/Input/InputActions/IA_DashRightShift.IA_DashRightShift"))
  ;[1 1 1] Handling dash for player 1.
  (:Triggered
    (Default|Dash (Utilities|Array|Get(acopy) (Variables|Default|Getplayers) 1))))

(event EventBeginPlay
  (Utilities|FlowControl|Delay 0.2)
  ;[1 1 1] Getting player start refs to set spawns.
  (bind _outactors (Actor|GetAllActorsOfClass "/Script/Engine.PlayerStart"))
  (Variables|Default|SetplayerStarts _outactors)
  ;[1 1 1] Getting player refs to control them.
  (bind _outactors_2 (Actor|GetAllActorsOfClass "/Game/Blueprints/Player/BP_Player.BP_Player_C"))
  (bind _output_get (Variables|Default|Setplayers _outactors_2))
  ;[1 1 1] Setting player refs to spawn at different player starts.
  (for (_array_element _array_index) _output_get
    (if (== _array_index 0)
      (Transformation|SetActorLocation _array_element (Transformation|GetActorLocation (Utilities|Array|Get(acopy) (Variables|Default|GetplayerStarts))) false false)
      (else
        (Transformation|SetActorLocation _array_element (Transformation|GetActorLocation (Utilities|Array|Get(acopy) (Variables|Default|GetplayerStarts) 1)) false false))))
  ;[1 1 1] Binding input mapping context to this player controller.
  (Input|AddMappingContext (PlayerController|LocalPlayerSubsystems|GetEnhancedInputLocalPlayerSubsystem self) "/Game/Blueprints/Player/Input/IMC_PlayerControls.IMC_PlayerControls" 0 "(bIgnoreAllPressedKeysUntilRelease=True,bForceImmediately=False)"))

(event EventTick
  (params (DeltaSeconds :type Float%20%28single-precision%29))
  (Variables|Default|SetdeltaTime DeltaSeconds))

(fn ConstructionScript)