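; Player controller for the main menu that lets two players sharing one keyboard change their choices.
; On BeginPlay it adds the menu controls Enhanced Input mapping context.
; The WASD and arrow-key move actions each pass their X axis value to BP_MainMenuGameMode's UpdatePlayerChoice, as the first and second player respectively.
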(event Input|EnhancedActionEvents|EnhancedInputActionIA_MoveArrows
  (params (ActionValue :type Vector%202D%20Structure) (ElapsedSeconds :type Float%20%28double-precision%29) (TriggeredSeconds :type Float%20%28double-precision%29) (InputAction :type Input%20Action%20Object%20Reference :default "/Game/Blueprints/Player/Input/InputActions/IA_MoveArrows.IA_MoveArrows"))
  (:Triggered
    (bind _asbp_main_menu_game_mode (Utilities|Casting|CastToBP_MainMenuGameMode (Game|GetGameMode)))
    (Default|UpdatePlayerChoice _asbp_main_menu_game_mode 1 (.X (Math|Vector2D|BreakVector2D ActionValue)))))

(event Input|EnhancedActionEvents|EnhancedInputActionIA_MoveWASD
  (params (ActionValue :type Vector%202D%20Structure) (ElapsedSeconds :type Float%20%28double-precision%29) (TriggeredSeconds :type Float%20%28double-precision%29) (InputAction :type Input%20Action%20Object%20Reference :default "/Game/Blueprints/Player/Input/InputActions/IA_MoveWASD.IA_MoveWASD"))
  (:Triggered
    (bind _asbp_main_menu_game_mode (Utilities|Casting|CastToBP_MainMenuGameMode (Game|GetGameMode)))
    (Default|UpdatePlayerChoice _asbp_main_menu_game_mode 0 (.X (Math|Vector2D|BreakVector2D ActionValue)))))

(event EventBeginPlay
  (Input|AddMappingContext (PlayerController|LocalPlayerSubsystems|GetEnhancedInputLocalPlayerSubsystem self) "/Game/Blueprints/Player/Input/IMC_MenuControls.IMC_MenuControls" 0 "(bIgnoreAllPressedKeysUntilRelease=True,bForceImmediately=False)"))

(event EventTick
  (params (DeltaSeconds :type Float%20%28single-precision%29)))

(fn ConstructionScript)